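; BP_CreepyFollower is an AI pawn that moves toward the player character when it sees or hears it.
; PawnSensing sight and noise events cast to the first-person, side-scroller and third-person characters, start AIMoveTo and print a debug label.
; DestroyMeSpecial spawns an explosion effect and sound, then destroys the actor.
; Any destruction increments the objects-destroyed count, but only when player 0 is the first-person character.
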(event OnSeePawn(PawnSensing)
  (params (Pawn :type Pawn%20Object%20Reference))
  (Utilities|FlowControl|Sequence
    (:then_0
      (bind _asbp_fp_char (Utilities|Casting|CastToBP_FP_Char Pawn))
      (AI|AIMoveTo self "0, 0, 0" _asbp_fp_char 5.0 false
        (:then
          (Development|PrintString "First"))))
    (:then_1
      (bind _asbp_ss_char (Utilities|Casting|CastToBP_SS_Char Pawn))
      (AI|AIMoveTo self "0, 0, 0" _asbp_ss_char 5.0 false
        (:then
          (Development|PrintString "Side"))))
    (:then_2
      (bind _asbp_tp_char (Utilities|Casting|CastToBP_TP_Char Pawn))
      (AI|AIMoveTo self "0, 0, 0" _asbp_tp_char 5.0 false
        (:then
          (Development|PrintString "Third"))))))

(event OnHearNoise(PawnSensing)
  (params (Instigator :type Pawn%20Object%20Reference) (Location :type Vector%20%28by%20ref%29 :default "0, 0, 0") (Volume :type Float%20%28single-precision%29))
  (Utilities|FlowControl|Sequence
    (:then_0
      (bind _asbp_fp_char (Utilities|Casting|CastToBP_FP_Char Instigator))
      (AI|AIMoveTo self "0, 0, 0" _asbp_fp_char 5.0 false
        (:then
          (Development|PrintString "First"))))
    (:then_1
      (bind _asbp_ss_char (Utilities|Casting|CastToBP_SS_Char Instigator))
      (AI|AIMoveTo self "0, 0, 0" _asbp_ss_char 5.0 false
        (:then
          (Development|PrintString "Side"))))
    (:then_2
      (bind _asbp_tp_char (Utilities|Casting|CastToBP_TP_Char Instigator))
      (AI|AIMoveTo self "0, 0, 0" _asbp_tp_char 5.0 false
        (:then
          (Development|PrintString "Third"))))))

(event EventDestroyed
  (CallFunction|IncrementDestroyCount))

(fn ConstructionScript)

(fn DestroyMeSpecial
  (bind _mesh (Variables|Character|GetMesh))
  (bind _returnvalue (Transformation|GetWorldLocation _mesh))
  (Effects|SpawnEmitteratLocation "/Game/StarterContent/Particles/P_Explosion.P_Explosion" _returnvalue)
  (Audio|PlaySoundatLocation "/Game/StarterContent/Audio/Explosion01.Explosion01" _returnvalue)
  (Actor|DestroyActor)
  (return))

(fn IncrementDestroyCount
  (bind _asbp_fp_char (Utilities|Casting|CastToBP_FP_Char (Game|GetPlayerCharacter 0))
    (:then
      (Default|IncrementObjectsDestroyed _asbp_fp_char))
    (:CastFailed
      _))
  (return))