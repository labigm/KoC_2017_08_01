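; BP_Barrel is a destructible barrel actor that exposes two ways to blow itself up.
; DestroyMeSpecial spawns the P_Explosion particle emitter at the Cylinder's location, while DestroyMeSparks spawns a BP_Sparks actor there instead.
; Both play the same explosion sound and then destroy the barrel; the file holds no trigger logic for either function.
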(fn ConstructionScript)

(fn DestroyMeSpecial
  (bind _cylinder (Variables|Default|GetCylinder))
  (bind _returnvalue (Transformation|GetWorldLocation _cylinder))
  (Effects|SpawnEmitteratLocation "/Game/StarterContent/Particles/P_Explosion.P_Explosion" _returnvalue)
  (Audio|PlaySoundatLocation "/Game/StarterContent/Audio/Explosion01.Explosion01" _returnvalue)
  (Actor|DestroyActor)
  (return))

(fn DestroyMeSparks
  (bind _cylinder (Variables|Default|GetCylinder))
  (bind _returnvalue (Transformation|GetWorldLocation _cylinder))
  (Game|SpawnActorfromClass "/Game/KoC/Blueprints/FirstPerson/BP_Sparks.BP_Sparks_C" (Math|Conversions|ToTransform(Vector) _returnvalue) "Undefined" 0 0)
  (Audio|PlaySoundatLocation "/Game/StarterContent/Audio/Explosion01.Explosion01" _returnvalue)
  (Actor|DestroyActor)
  (return))