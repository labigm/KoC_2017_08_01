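; Explodable cube actor that destroys itself with an explosion emitter and a spawned BP_Sparks actor at its location.
; Any actor overlap triggers this directly, while hits trigger it only for egg, light or submachine bullets.
; The ShouldDestroy macro filters hits through a cast chain and also destroys the matching bullet.
; On Destroyed, it casts the player character to BP_FP_Char and increments its destroyed-object count.
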(event Collision|EventActorBeginOverlap
  (params (OtherActor :type Actor%20Object%20Reference))
  (bind _returnvalue (Transformation|GetActorLocation))
  (Actor|DestroyActor)
  (Effects|SpawnEmitteratLocation "/Game/StarterContent/Particles/P_Explosion.P_Explosion" _returnvalue)
  (Game|SpawnActorfromClass "/Game/KoC/Blueprints/FirstPerson/BP_Sparks.BP_Sparks_C" (Math|Conversions|ToTransform(Vector) _returnvalue) "Undefined" 0 0))

(event Collision|EventHit
  (params (MyComp :type Primitive%20Component%20Object%20Reference) (Other :type Actor%20Object%20Reference) (OtherComp :type Primitive%20Component%20Object%20Reference) (bSelfMoved :type Boolean) (HitLocation :type Vector :default "0, 0, 0") (HitNormal :type Vector :default "0, 0, 0") (NormalImpulse :type Vector :default "0, 0, 0") (Hit :type Hit%20Result%20Structure%20%28by%20ref%29))
  (bind _returnvalue (Transformation|GetActorLocation))
  (Utilities|ShouldDestroy Other
    (:Destroy
      (Actor|DestroyActor)
      (Effects|SpawnEmitteratLocation "/Game/StarterContent/Particles/P_Explosion.P_Explosion" _returnvalue)
      (Game|SpawnActorfromClass "/Game/KoC/Blueprints/FirstPerson/BP_Sparks.BP_Sparks_C" (Math|Conversions|ToTransform(Vector) _returnvalue) "Undefined" 0 0))))

(event EventDestroyed
  (CallFunction|IncrementDestroyCount))

(fn ConstructionScript)

(fn IncrementDestroyCount
  (bind _asbp_fp_char (Utilities|Casting|CastToBP_FP_Char (Game|GetPlayerCharacter 0))
    (:then
      (Default|IncrementObjectsDestroyed _asbp_fp_char))
    (:CastFailed
      _))
  (return))